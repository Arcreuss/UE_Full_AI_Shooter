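; Player pawn Blueprint for a third-person shooter that maps input to movement, look, firing, combat stance, sprint, crouch and aim-down-sights.
; Input events forward to functions defined outside these graphs, with sprint and fire held and equip, crouch and ADS toggled from AnimValues flags.
; ADS also runs a Zoom In/Out graph, whose timeline plays or reverses to blend spring arm length, socket offset and camera FOV.
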(event EventBeginPlay
  (|CallParentFunction) ; This node is disabled and will not be called.\nDrag off pins to build functionality.
)

(event Collision|EventActorBeginOverlap
  (params (OtherActor :type Actor%20Object%20Reference))
  (|CallParentFunction OtherActor) ; This node is disabled and will not be called.\nDrag off pins to build functionality.
)

(event EventTick
  (params (DeltaSeconds :type Float%20%28single-precision%29))
  (|CallParentFunction DeltaSeconds) ; This node is disabled and will not be called.\nDrag off pins to build functionality.
)

(event Input|ActionEvents|InputActionEquipWeapon
  (params (Key :type Key%20Structure :default "None"))
  ;[0 0 0] Inputs
  (:Pressed
    (Class|CharacterBase|ToggleCombat (not (.bisincombat (Variables|Default|GetAnimValues))))))

(event Input|ActionEvents|InputActionSprint
  (params (Key :type Key%20Structure :default "None"))
  ;[0 0 0] Inputs
  (:Pressed
    (Class|CharacterBase|ToggleSprinting true))
  (:Released
    (Class|CharacterBase|ToggleSprinting false)))

(event Input|ActionEvents|InputActionCrouch
  (params (Key :type Key%20Structure :default "None"))
  ;[0 0 0] Inputs
  (:Pressed
    (Class|CharacterBase|ToggleCrouch (not (.biscrouching (Variables|Default|GetAnimValues))))))

(event Input|ActionEvents|InputActionADS
  (params (Key :type Key%20Structure :default "None"))
  (bind _animvalues (Variables|Default|GetAnimValues))
  ;[0 0 0] Inputs
  (:Pressed
    (Class|CharacterBase|ToggleADS (not (.bads _animvalues)))
    (|ZoomIn/Out (.bads _animvalues))))

(event Input|ActionEvents|InputActionFire
  (params (Key :type Key%20Structure :default "None"))
  ;[0 0 0] Inputs
  (:Pressed
    (Class|CharacterBase|StartWeaponFire))
  (:Released
    (Class|CharacterBase|StopWeaponFire)))

(event Input|AxisEvents|InputAxisMoveForward
  (params (AxisValue :type Float%20%28single-precision%29))
  ;[0 0 0] Inputs
  (Class|CharacterBase|MoveForward AxisValue))

(event Input|AxisEvents|InputAxisMoveRight
  (params (AxisValue :type Float%20%28single-precision%29))
  ;[0 0 0] Inputs
  (Class|CharacterBase|MoveRight AxisValue))

(event Input|AxisEvents|InputAxisTurn
  (params (AxisValue :type Float%20%28single-precision%29))
  ;[0 0 0] Inputs
  (Class|CharacterBase|Turn AxisValue))

(event Input|AxisEvents|InputAxisLookUp
  (params (AxisValue :type Float%20%28single-precision%29))
  ;[0 0 0] Inputs
  (Class|CharacterBase|LookUp AxisValue))

(fn ConstructionScript
  (|CallParentFunction))