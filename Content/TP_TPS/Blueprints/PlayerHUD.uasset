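; Third-person shooter player HUD that draws a dynamic white crosshair at screen center while a player character exists.
; DrawHUD renders four bars and a center dot with DrawRect calls.
; Length sets the bar size, while the gap is Accuracy plus a capped amount scaled from character velocity, so the crosshair spreads as the player moves faster.
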(event EventDrawHUD
  (params (SizeX :type Integer) (SizeY :type Integer))
  (bind _returnvalue (Game|GetPlayerCharacter 0))
  (bind _returnvalue_2 (/ SizeX 2))
  (bind _returnvalue_3 (/ SizeY 2))
  (bind _accuracy (Variables|Default|GetAccuracy))
  (bind _length (Variables|Default|GetLength))
  (bind _length_2 (Variables|Default|GetLength))
  (bind _returnvalue_4 (Transformation|GetVelocity _returnvalue))
  (bind _returnvalue_5 (Math|Conversions|ToFloat(Integer) _returnvalue_2))
  (bind _returnvalue_6 (Math|Conversions|ToFloat(Integer) _returnvalue_3))
  (bind _returnvalue_7 (Math|Vector|VectorLength _returnvalue_4))
  (bind _returnvalue_8 (/ _returnvalue_7 8.0))
  (bind _returnvalue_9 (Math|Float|Min(Float) _returnvalue_8 4e+01))
  (bind _returnvalue_10 (+ _accuracy _returnvalue_9))
  (Utilities|IsValid (Game|GetPlayerCharacter 0)
    (:Is%20Valid
      (Utilities|FlowControl|Sequence
        (:then_0
          (HUD|DrawRect "(R=1.000000,G=1.000000,B=1.000000,A=1.000000)" (- (- _returnvalue_5 _returnvalue_10) (Variables|Default|GetLength)) _returnvalue_6 _length 3.0)
          (HUD|DrawRect "(R=1.000000,G=1.000000,B=1.000000,A=1.000000)" (+ _returnvalue_10 _returnvalue_5) _returnvalue_6 _length 3.0)
          (HUD|DrawRect "(R=1.000000,G=1.000000,B=1.000000,A=1.000000)" _returnvalue_5 (- (- _returnvalue_6 _returnvalue_10) _length_2) 3.0 _length_2)
          (HUD|DrawRect "(R=1.000000,G=1.000000,B=1.000000,A=1.000000)" _returnvalue_5 (+ _returnvalue_10 _returnvalue_6) 3.0 _length_2))
        (:then_1
          (HUD|DrawRect "(R=1.000000,G=1.000000,B=1.000000,A=1.000000)" _returnvalue_5 _returnvalue_6 3.0 3.0))))))

(fn ConstructionScript)